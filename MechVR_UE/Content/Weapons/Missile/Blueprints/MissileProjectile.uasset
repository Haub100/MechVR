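; Homing missile projectile actor that chases a target and explodes on contact.
; HomingMissle starts the sound, sets a lifespan and configures projectile homing toward the target's static mesh.
; Tick turns the missile toward the target with RInterpTo, easing the turn speed through FInterpTo to avoid snapping at launch.
; The first hit fires an impulse, plays explosion effects and removes missile components, destroying the smoke trail after a delay.
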(event `MissileAngle`
  (params (HomingTarget :type "StaticMeshComponent Object Reference"))
  (bind _returnvalue (`KismetMathLibrary.FInterpTo` (`self.RocketRotSpeed`) (`self.RocketTargetRotSpeed`) (`GameplayStatics.GetWorldDeltaSeconds`) 2.0))
  ;[1 1 1] MissleRotator
  (if (`KismetSystemLibrary.IsValid` HomingTarget)
    (set `self.RocketRotSpeed` _returnvalue) ; Set current rotation speed\nin order to make Finterp work
    (`self.K2_SetActorRotation` (`KismetMathLibrary.RInterpTo` (`self.K2_GetActorRotation`) (`KismetMathLibrary.FindLookAtRotation` (`self.K2_GetActorLocation`) (`SceneComponent.K2_GetComponentLocation` HomingTarget)) (`GameplayStatics.GetWorldDeltaSeconds`) _returnvalue)) ; Rotate rocket toward Target
  ))

(event `self.CollisionComponent.OnComponentHit`
  (params (HitComponent :type "PrimitiveComponent Object Reference") (OtherActor :type "Actor Object Reference") (OtherComp :type "PrimitiveComponent Object Reference") (NormalImpulse :type "Vector Structure") (Hit :type "HitResult Structure (by ref)"))
  (bind _r (`self.r`))
  (bind _returnvalue (`SceneComponent.K2_GetComponentLocation` _r))
  ;[1 1 1] Explode on contact
  (`/Engine/EditorBlueprintResources/StandardMacros.DoOnce` false
    (:`Completed`
      (`RadialForceComponent.FireImpulse` _r)
      (`GameplayStatics.PlaySoundAtLocation` "/Game/StarterContent/Audio/Explosion01.Explosion01" _returnvalue)
      (`AudioComponent.Stop` (`self.MissileSound`))
      (`GameplayStatics.SpawnEmitterAtLocation` "/Game/StarterContent/Particles/P_Explosion.P_Explosion" _returnvalue)
      (`ActorComponent.K2_DestroyComponent` (`self.Projectile`))
      (`ActorComponent.K2_DestroyComponent` (`self.Missile`))
      (`ActorComponent.K2_DestroyComponent` (`self.Glow`))
      (`ActorComponent.K2_DestroyComponent` (`self.Warhead`))
      (`KismetSystemLibrary.Delay` 2.0)
      (`ActorComponent.K2_DestroyComponent` (`self.SmokeTrail`)))))

(event `HomingMissle`
  (params (TargetToHit :type "StaticMeshActor Object Reference"))
  (bind _projectile (`self.Projectile`))
  ;[1 1 1] Set Homing Missle
  (`AudioComponent.Play` (`self.MissileSound`) 0.0)
  (`self.SetLifeSpan` 8.0)
  (if (`KismetSystemLibrary.IsValid` TargetToHit)
    (set `ProjectileMovementComponent.HomingTargetComponent` (`StaticMeshActor.StaticMeshComponent` TargetToHit) _projectile)
    (set `ProjectileMovementComponent.bIsHomingProjectile` true _projectile)
    (set `ProjectileMovementComponent.HomingAccelerationMagnitude` 5000.0 _projectile)))

(event `self.ReceiveTick`
  (params (DeltaSeconds :type "Float (single-precision)"))
  ;[1 1 1] Set Homing Missle
  (if (`KismetSystemLibrary.IsValid` (stale `HomingMissle` TargetToHit))
    (`self.MissileAngle` (`StaticMeshActor.StaticMeshComponent` (stale `HomingMissle` TargetToHit)))))

(fn `UserConstructionScript`)