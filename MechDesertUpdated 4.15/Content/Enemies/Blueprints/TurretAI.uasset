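; Enemy tank turret AI that turns its base and top toward the player and fires on a tick counter once PawnSensing spots them.
; FireTank alternates explosion effects between two gun sockets, resting after each pair, while ShellImpact fakes shells with explosions at random reachable points near the player.
; Component hits from minigun, missile and tank projectiles reduce Health, shown on a widget bar, destroying the actor at zero.
; Tank movement logic is disconnected.
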(event `self.ReceiveTick`
  (params (DeltaSeconds :type "Float (single-precision)"))
  (`|ExecutionSequence`
    (:`then_0`
      (if (`self.SeesPlayer`)
        (`|ExecutionSequence`
          (:`then_0`
            (`self.RotateTop`))
          (:`then_1`
            (`self.RotateBottom`))
          (:`then_2`
            (bind _result (`/Engine/EditorBlueprintResources/StandardMacros.IncrementInt` (`self.FireTimer`))
              (:`  `
                (bind _output_get (set `self.FireTimer` _result))
                (bind _returnvalue (>= _output_get 50))
                (if (and _returnvalue (`self.Rest`))
                  (`KismetSystemLibrary.Delay` 1.0)
                  (set `self.FireTimer` 0)
                  (set `self.Rest` false)
                  (elif _returnvalue
                    (set `self.FireTimer` 0)
                    (`self.FireTank` self)
                    (`KismetSystemLibrary.Delay` 0.3)
                    (`self.ShellImpact`)
                    (if (not (`self.WhichGun`))
                      (set `self.Rest` true))))))))))
    (:`then_1`
      (bind _asai_health (cast `/Game/Enemies/AI_Health` (`WidgetComponent.GetUserWidgetObject` (`self.HealthBar`))))
      (`ProgressBar.SetPercent` (`/Game/Enemies/AI_Health.ProgressBar_36` _asai_health) (/ (`self.Health`) 100.0)))))

(event `self.PawnSensing.OnSeePawn`
  (params (Pawn :type "Pawn Object Reference"))
  (set `self.SeesPlayer` (== Pawn (`GameplayStatics.GetPlayerCharacter` 0))))

(event `Die_Event`
  ;[1 1 1] Health and Damage
  (`self.K2_DestroyActor`))

(event `DamageMinigun_Event`
  ;[1 1 1] Health and Damage
  (bind _output_get (set `self.Health` (- (`self.Health`) 5.0)))
  (if (<= _output_get 0.0)
    (`self.Die_Event`)))

(event `DamageMissile_Event`
  ;[1 1 1] Health and Damage
  (bind _output_get (set `self.Health` (- (`self.Health`) 40.0)))
  (if (<= _output_get 0.0)
    (`self.Die_Event`)))

(event `DamageTankGun_Event`
  ;[1 1 1] Health and Damage
  (bind _output_get (set `self.Health` (- (`self.Health`) 50.0)))
  (if (<= _output_get 0.0)
    (`self.Die_Event`)))

(event `self.Collider.OnComponentHit`
  (params (HitComponent :type "PrimitiveComponent Object Reference") (OtherActor :type "Actor Object Reference") (OtherComp :type "PrimitiveComponent Object Reference") (NormalImpulse :type "Vector Structure") (Hit :type "HitResult Structure (by ref)"))
  ;[1 1 1] Health and Damage
  (if (== (`GameplayStatics.GetObjectClass` OtherActor) "/Game/Weapons/Minigun/Blueprints/MinigunProjectile.MinigunProjectile_C")
    (`self.DamageMinigun_Event`)
    (elif (== OtherActor "/Game/Weapons/Missile/Blueprints/MissileProjectile.MissileProjectile")
      (`self.DamageMissile_Event`)
      (elif (== (`GameplayStatics.GetObjectClass` OtherActor) "/Game/Weapons/TankGun/Blueprints/TankGunProjectile.TankGunProjectile_C")
        (`self.DamageTankGun_Event`)))))

(event `self.Base.OnComponentHit`
  (params (HitComponent :type "PrimitiveComponent Object Reference") (OtherActor :type "Actor Object Reference") (OtherComp :type "PrimitiveComponent Object Reference") (NormalImpulse :type "Vector Structure") (Hit :type "HitResult Structure (by ref)"))
  ;[1 1 1] Health and Damage
  (`KismetSystemLibrary.PrintString` (`KismetStringLibrary.Conv_ObjectToString` HitComponent))
  (`KismetSystemLibrary.PrintString` (`KismetSystemLibrary.GetDisplayName` OtherActor))
  (`KismetSystemLibrary.PrintString` (`KismetSystemLibrary.GetDisplayName` OtherComp))
  (if (== OtherActor "/Game/Weapons/Minigun/Blueprints/MinigunProjectile.MinigunProjectile")
    (`self.DamageMinigun_Event`)
    (elif (== OtherActor "/Game/Weapons/Missile/Blueprints/MissileProjectile.MissileProjectile")
      (`self.DamageMissile_Event`)
      (elif (== OtherActor "/Game/Weapons/TankGun/Blueprints/TankGunProjectile.TankGunProjectile")
        (`self.DamageTankGun_Event`)))))

(event `self.Top.OnComponentHit`
  (params (HitComponent :type "PrimitiveComponent Object Reference") (OtherActor :type "Actor Object Reference") (OtherComp :type "PrimitiveComponent Object Reference") (NormalImpulse :type "Vector Structure") (Hit :type "HitResult Structure (by ref)"))
  ;[1 1 1] Health and Damage
  (if (== OtherActor "/Game/Weapons/Minigun/Blueprints/MinigunProjectile.MinigunProjectile")
    (`self.DamageMinigun_Event`)
    (elif (== OtherActor "/Game/Weapons/Missile/Blueprints/MissileProjectile.MissileProjectile")
      (`self.DamageMissile_Event`)
      (elif (== OtherActor "/Game/Weapons/TankGun/Blueprints/TankGunProjectile.TankGunProjectile")
        (`self.DamageTankGun_Event`)))))

(event `self.Guns.OnComponentHit`
  (params (HitComponent :type "PrimitiveComponent Object Reference") (OtherActor :type "Actor Object Reference") (OtherComp :type "PrimitiveComponent Object Reference") (NormalImpulse :type "Vector Structure") (Hit :type "HitResult Structure (by ref)"))
  ;[1 1 1] Health and Damage
  (if (== OtherActor "/Game/Weapons/Minigun/Blueprints/MinigunProjectile.MinigunProjectile")
    (`self.DamageMinigun_Event`)
    (elif (== OtherActor "/Game/Weapons/Missile/Blueprints/MissileProjectile.MissileProjectile")
      (`self.DamageMissile_Event`)
      (elif (== OtherActor "/Game/Weapons/TankGun/Blueprints/TankGunProjectile.TankGunProjectile")
        (`self.DamageTankGun_Event`)))))

(fn `FireTank`
  (if (not (`self.WhichGun`))
    (`|SpawnActorFromClass` "/Game/StarterContent/Blueprints/Blueprint_Effect_ExplosionSmall.Blueprint_Effect_ExplosionSmall_C" (`SceneComponent.GetSocketTransform` (`self.Guns`) "RIGHT" "RTS_World") "Undefined" "OverrideRootScale")
    (set `self.WhichGun` true)
    (else
      (`|SpawnActorFromClass` "/Game/StarterContent/Blueprints/Blueprint_Effect_Explosion.Blueprint_Effect_Explosion_C" (`SceneComponent.GetSocketTransform` (`self.Guns`) "LEFT" "RTS_World") "Undefined" "OverrideRootScale")
      (set `self.WhichGun` false))))

(fn `MoveTank`)

(fn `RotateBottom`
  (bind _base (`self.Base`))
  (bind (_returnvalue_roll _returnvalue_pitch _returnvalue_yaw) (`KismetMathLibrary.BreakRotator` (`SceneComponent.K2_GetComponentRotation` _base)))
  ;[1 1 1] Rotates bottom of tank towards player
  (`SceneComponent.K2_SetWorldRotation` _base (`KismetMathLibrary.FindLookAtRotation` (`self.K2_GetActorLocation` (`GameplayStatics.GetPlayerCharacter` 0)) (`self.K2_GetActorLocation` (`ActorComponent.GetOwner` _base))) false false)
  (`SceneComponent.K2_SetWorldRotation` _base (`KismetMathLibrary.MakeRotator` (+ _returnvalue_roll 90.0) 0.0 (- _returnvalue_yaw 180.0)) false false))

(fn `RotateTop`
  (bind _top (`self.Top`))
  (bind (_returnvalue_roll _returnvalue_pitch _returnvalue_yaw) (`KismetMathLibrary.BreakRotator` (`SceneComponent.K2_GetComponentRotation` _top)))
  ;[1 1 1] Rotates turret towards the player
  (`SceneComponent.K2_SetWorldRotation` _top (`KismetMathLibrary.FindLookAtRotation` (`self.K2_GetActorLocation` (`GameplayStatics.GetPlayerCharacter` 0)) (`self.K2_GetActorLocation` (`ActorComponent.GetOwner` _top))) false false)
  (`SceneComponent.K2_SetWorldRotation` _top (`KismetMathLibrary.MakeRotator` (+ _returnvalue_roll 90.0) (+ _returnvalue_pitch 0.0) (- _returnvalue_yaw 0.0)) false false))

(fn `ShellImpact`
  (`|SpawnActorFromClass` "/Game/StarterContent/Blueprints/Blueprint_Effect_Explosion.Blueprint_Effect_Explosion_C" (`KismetMathLibrary.MakeTransform` (`NavigationSystem.GetRandomReachablePointInRadius` (`self.K2_GetActorLocation` (`GameplayStatics.GetPlayerCharacter` 0)) 500.0) (`KismetMathLibrary.RandomRotator` false)) "Undefined" "OverrideRootScale"))

(fn `UserConstructionScript`
  (`self.SpawnDefaultController` self))