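; Enemy tank AI that starts chasing and shelling the player once pawn sensing spots a character.
; AIMoveTo drives the approach, while Tick rotates turret and hull toward the player and fires on a frame-counted timer.
; Shots have no projectile: an explosion spawns at the cannon tip, then another at a random reachable point near the player after a delay.
; SeesPlayer never resets, and MoveTank holds only disconnected movement code.
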(event `self.ReceiveTick`
  (params (DeltaSeconds :type "Float (single-precision)"))
  (if (`self.SeesPlayer`)
    (`|ExecutionSequence`
      (:`then_0`
        (`self.RotateTop`))
      (:`then_1`
        (`self.RotateBottom` self))
      (:`then_3`
        (bind _result (`/Engine/EditorBlueprintResources/StandardMacros.IncrementInt` (`self.FireTimer`))
          (:`  `
            (bind _output_get (set `self.FireTimer` _result))
            (if (>= _output_get 180)
              (`KismetSystemLibrary.PrintString` "FIR!")
              (set `self.FireTimer` 0)
              (`self.FireTank` self)
              (`KismetSystemLibrary.Delay` 0.3)
              (`self.ShellImpact`))))))))

(event `self.PawnSensing.OnSeePawn`
  (params (Pawn :type "Pawn Object Reference"))
  (set `self.SeesPlayer` true)
  (bind _ascharacter (cast `Character` Pawn))
  (`|AIMoveTo` self (0.0 0.0 0.0) _ascharacter 1000.0))

(fn `FireTank`
  (`|SpawnActorFromClass` "/Game/StarterContent/Blueprints/Blueprint_Effect_Explosion.Blueprint_Effect_Explosion_C" (`SceneComponent.GetSocketTransform` (`self.TankTop`) "CANNON_TIP" "RTS_World") "Undefined" "OverrideRootScale"))

(fn `MoveTank`)

(fn `RotateBottom`
  (bind _tankbottom (`self.TankBottom`))
  (bind (_returnvalue_roll _returnvalue_pitch _returnvalue_yaw) (`KismetMathLibrary.BreakRotator` (`SceneComponent.K2_GetComponentRotation` _tankbottom)))
  ;[1 1 1] Rotates bottom of tank towards player
  (`SceneComponent.K2_SetWorldRotation` _tankbottom (`KismetMathLibrary.FindLookAtRotation` (`self.K2_GetActorLocation` (`GameplayStatics.GetPlayerCharacter` 0)) (`self.K2_GetActorLocation` (`ActorComponent.GetOwner` _tankbottom))) false false)
  (`SceneComponent.K2_SetWorldRotation` _tankbottom (`KismetMathLibrary.MakeRotator` 0.0 0.0 _returnvalue_yaw) false false))

(fn `RotateTop`
  (bind _tanktop (`self.TankTop`))
  (bind (_returnvalue_roll _returnvalue_pitch _returnvalue_yaw) (`KismetMathLibrary.BreakRotator` (`SceneComponent.K2_GetComponentRotation` _tanktop)))
  ;[1 1 1] Rotates turret towards the player
  (`SceneComponent.K2_SetWorldRotation` _tanktop (`KismetMathLibrary.FindLookAtRotation` (`self.K2_GetActorLocation` (`GameplayStatics.GetPlayerCharacter` 0)) (`self.K2_GetActorLocation` (`ActorComponent.GetOwner` (`self.TankTop`)))) false false)
  (`SceneComponent.K2_SetWorldRotation` _tanktop (`KismetMathLibrary.MakeRotator` 0.0 (+ _returnvalue_pitch 7.0) _returnvalue_yaw) false false))

(fn `ShellImpact`
  (`|SpawnActorFromClass` "/Game/StarterContent/Blueprints/Blueprint_Effect_Explosion.Blueprint_Effect_Explosion_C" (`KismetMathLibrary.MakeTransform` (`NavigationSystem.GetRandomReachablePointInRadius` (`self.K2_GetActorLocation` (`GameplayStatics.GetPlayerCharacter` 0)) 500.0) (`KismetMathLibrary.RandomRotator` false)) "Undefined" "OverrideRootScale"))

(fn `UserConstructionScript`)